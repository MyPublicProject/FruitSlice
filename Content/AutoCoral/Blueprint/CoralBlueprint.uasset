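; Construction-script actor that builds an underwater reef area, with an optional water surface and procedurally scattered coral.
; Water offsets the mesh, tints post-process settings and feeds a dynamic material.
; For each CoralMembers entry, CoralMacro fires random downward traces from the Box bounds, filtering hits by depth, optionally retrying.
; Accepted hits spawn instanced or individual meshes with random scale, yaw and Z offset, optional normal alignment and collision.
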(fn `UserConstructionScript`
  (bind _watermaterial (`self.WaterMaterial`))
  (bind _underwatercolor (`self.UnderwaterColor`))
  (bind _gamma (`self.Gamma`))
  (`|ExecutionSequence`
    (:`then_0`
      (if (`self.Water`)
        ;[0 0 0] Water Offset/Visibility
        (`SceneComponent.K2_AddLocalOffset` (`self.WaterMesh`) (* (0.0 0.0 1.0) (`self.WaterOffset`)) false false)
        ;[0 0 0] Setting texture parameters and post process
        (`PrimitiveComponent.SetMaterial` (`self.WaterMesh`) 0 (`self.Material`))
        (if (`self.UseSurfaceColor`)
          (set `self.UnderwaterColor` (`self.Overall Color`)))
        (setmembers `PostProcessSettings` :`StructRef` (`PostProcessComponent.Settings` (`self.PostProcess`)) :`ColorGamma` (`KismetMathLibrary.MakeVector4` _gamma _gamma _gamma 1.0) :`FilmWhitePoint` _underwatercolor :`SceneColorTint` _underwatercolor :`SceneFringeIntensity` (`self.Fringe`) :`BloomIntensity` (`self.Bloom Intensity`) :`BloomThreshold` (`self.Bloom Threshold`) :`VignetteIntensity` (`self.VignetteIntensity`))
        (bind _returnvalue (`PrimitiveComponent.CreateDynamicMaterialInstance` (`self.WaterMesh`) 0 null))
        (set `self.WaterMaterial` _returnvalue)
        (`MaterialInstanceDynamic.SetScalarParameterValue` _watermaterial "TilingU" (.x (`self.GetActorScale3D`)))
        (`MaterialInstanceDynamic.SetScalarParameterValue` _watermaterial "Tilingv" (.y (`self.GetActorScale3D`)))
        (`MaterialInstanceDynamic.SetScalarParameterValue` _watermaterial "Tiling" (`self.Tiling`))
        (`MaterialInstanceDynamic.SetScalarParameterValue` _watermaterial "WaterOpacity" (`self.Opacity`))
        (`MaterialInstanceDynamic.SetScalarParameterValue` _watermaterial "FadeDistance" (`self.FadeDistance`))
        (`MaterialInstanceDynamic.SetScalarParameterValue` _watermaterial "Metallic" (`self.Metallic`))
        (`MaterialInstanceDynamic.SetScalarParameterValue` _watermaterial "Roughness" (`self.Roughness`))
        (`MaterialInstanceDynamic.SetScalarParameterValue` _watermaterial "RippleSpeed" (`self.RippleSpeed`))
        (`MaterialInstanceDynamic.SetScalarParameterValue` _watermaterial "RefractionWarp" (`self.RefractionWarp`))
        (`MaterialInstanceDynamic.SetScalarParameterValue` _watermaterial "RefractionContrast" (`self.RefractionContrast`))
        (`MaterialInstanceDynamic.SetVectorParameterValue` _watermaterial "Color" (`self.Overall Color`))
        (`MaterialInstanceDynamic.SetVectorParameterValue` _watermaterial "FresnelColor1" (`self.FresnelColor1`))
        (`MaterialInstanceDynamic.SetVectorParameterValue` _watermaterial "FresnelColor2" (`self.FresnelColor2`))
        (`MaterialInstanceDynamic.SetTextureParameterValue` _watermaterial "RippleNormal" (`self.Ripple Normal`))
        (`MaterialInstanceDynamic.SetTextureParameterValue` _watermaterial "ReflectionTexture" (`self.ReflectionVector`))
        (else
          (`SceneComponent.SetVisibility` (`self.WaterMesh`) false true)
          (`SceneComponent.SetVisibility` (`self.Box`) true false))))
    (:`then_1`
      ;[0 0 0] Coral System
      (if (`self.CoralSystem`)
        (if (`self.RefreshCoralSystem`)
          _
          (else
            _))
        (set `self.RefreshCoralSystem` false)
        (for _array_element (`self.CoralMembers`)
          (bind (_coral _frequency _scale _scalevariation _depth _reversedepth_ _zoffset _randomzoffset _normalalign_ _collision_) (break `/Game/AutoCoral/Blueprint/CoralStruct` _array_element))
          (`self.CoralMacro` _coral _frequency _scale _scalevariation _depth _reversedepth_ _zoffset _randomzoffset _normalalign_ _collision_))))))